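; BP_Door is an interactable door that swings open away from or toward a side chosen by the player's position, and closes on the next interaction.
; Interaction toggles a closed flag, playing or reversing a timeline that lerps the Door component's relative yaw.
; On opening, the dot product of the player-to-door direction and the actor's right vector picks a positive or negative swing.
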(event Custom|OpenCloseDoor
  (bind _self self)
  (if (Variables|Default|GetDoorClosed?)
    (Variables|Default|SetDoorClosed? false)
    (Variables|Default|SetDotProduct (Math|Vector|DotProduct (Math|Vector|Normalize (- (Transformation|GetActorLocation _self) (Transformation|GetActorLocation (Variables|Default|GetPlayerRef)))) (Transformation|GetActorRightVector _self)))
    (bind _alpha (Timeline|Door_TL Play)
      (:Update
        (Transformation|SetRelativeRotation (Variables|Default|GetDoor) (Math|Rotator|MakeRotator 0.0 0.0 (Math|Float|Lerp 0.0 (Math|Float|SelectFloat 85.0 -85.0 (>= (Variables|Default|GetDotProduct) 0.0)) _alpha)) false false)))
    (else
      (Variables|Default|SetDoorClosed? true)
      (Timeline|Door_TL Reverse))))

(event EventBeginPlay
  (bind _asbp_third_person_character (Utilities|Casting|CastToBP_ThirdPersonCharacter (Game|GetPlayerCharacter 0)))
  (Variables|Default|SetPlayerRef _asbp_third_person_character))

(event EventInteraction
  (CallFunction|OpenCloseDoor))

(fn ConstructionScript)