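; BP_PuzzleSlab is a floor tile in a slab puzzle that must be stepped on only once.
; On BeginPlay it caches the BP_Slab_PuzzleManager found in the level.
; A first overlap lights the slab material, plays a cue, marks it active and asks the manager to check completion.
; Overlapping an active slab tells the manager to reset the puzzle with a denied buzzer, while ResetTile restores the unlit state.
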(event Custom|ResetTile
  (Variables|Default|SetIsActive false)
  (Rendering|Material|SetMaterial (Variables|Default|GetSlabMesh_0) 0 "/Game/Materials/MI_SlabTexture.MI_SlabTexture"))

(event EventBeginPlay
  (bind _outactors (Actor|GetAllActorsOfClass "/Game/Blueprints/Slab_Puzzle/BP_Slab_PuzzleManager.BP_Slab_PuzzleManager_C"))
  (for _array_element _outactors
    (Variables|Default|SetPuzzleManagerRef _array_element)))

(event Collision|EventActorBeginOverlap
  (params (OtherActor :type Actor%20Object%20Reference))
  (if (Variables|Default|GetIsActive)
    (Class|BIPuzzleComm|ResetPuzzle(Message) (Variables|Default|GetPuzzleManagerRef))
    (Audio|PlaySoundatLocation "/Game/Audio/419023__jacco18__acess-denied-buzz.419023__jacco18__acess-denied-buzz" "0, 0, 0" "0, 0, 0" 1.0 1.0 0.0 0 0 0 0)
    (else
      (Rendering|Material|SetMaterial (Variables|Default|GetSlabMesh_0) 0 "/Game/Materials/MI_LitSlab.MI_LitSlab")
      (Audio|PlaySoundatLocation "/Game/Audio/SlabCue.SlabCue" (Transformation|GetActorLocation) "0, 0, 0" 1.0 1.0 0.0 0 0 0 0)
      (Variables|Default|SetIsActive true)
      (Class|BIPuzzleComm|CheckPuzzleCompletion(Message) (Variables|Default|GetPuzzleManagerRef)))))

(fn ConstructionScript)