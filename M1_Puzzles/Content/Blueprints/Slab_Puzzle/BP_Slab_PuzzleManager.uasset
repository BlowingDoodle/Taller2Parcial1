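; Puzzle manager for the slab puzzle, tracking progress and opening a door when it is solved.
; On BeginPlay it gathers and counts every BP_PuzzleSlab in the level and caches the BP_Player.
; Each CheckPuzzleCompletion call increments a counter; reaching the slab count toggles SlabDoorRef and shows the player's win message.
; ResetPuzzle shows an incorrect message, resets all slabs and zeroes the counter.
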(event EventBeginPlay
  (bind _outactors (Actor|GetAllActorsOfClass "/Game/Blueprints/Slab_Puzzle/BP_PuzzleSlab.BP_PuzzleSlab_C"))
  (bind _output_get (Variables|Default|SetpuzzleSlabs _outactors))
  (for _array_element _output_get
    (bind _result (Math|Integer|IncrementInt (Variables|Default|GetSlabsCount))
      (:%20%20
        (Variables|Default|SetSlabsCount _result)
        (bind _outactors_2 (Actor|GetAllActorsOfClass "/Game/Blueprints/BP_Player.BP_Player_C"))
        ;[1 1 1] Debug
        (for _array_element_2 _outactors_2
          (Variables|Default|SetPlayerRef _array_element_2))))))

(event Collision|EventActorBeginOverlap
  (params (OtherActor :type Actor%20Object%20Reference)))

(event EventTick
  (params (DeltaSeconds :type Float%20%28single-precision%29)))

(event EventResetPuzzle
  (Class|BPIPlayerActions|IncorrectPuzzle(Message) (Variables|Default|GetPlayerRef))
  (for _array_element (Variables|Default|GetpuzzleSlabs)
    (Default|ResetTile _array_element)
    (Variables|Default|SetCompletionIndex 0)))

(event EventCheckPuzzleCompletion
  (bind _result (Math|Integer|IncrementInt (Variables|Default|GetCompletionIndex))
    (:%20%20
      (bind _output_get (Variables|Default|SetCompletionIndex _result))
      (if (>= _output_get (Variables|Default|GetSlabsCount))
        (Default|OpenCloseDoor (Variables|Default|GetSlabDoorRef))
        (Class|BPIPlayerActions|WinPuzzle(Message) (Variables|Default|GetPlayerRef))))))

(fn ConstructionScript)