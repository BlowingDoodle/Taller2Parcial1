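; Double slab door for the slab puzzle, with a point light that randomly starts either steady or flickering.
; OpenCloseDoor swings both leaves open on a timeline in a fixed direction, playing a sound and re-randomizing the light in its open color on each update.
; Closing only sets the DoorClosed flag; distance-based auto-close and player-relative swing logic are left unwired.
; Interaction plays a metal door sound and stops a second timeline.
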(event Custom|OpenCloseDoor
  ;[0 0.02053 1 0.5] Door Animation
  (if (Variables|Default|GetDoorClosed?)
    (Variables|Default|SetDoorClosed? false)
    ;;[0.15 0.15 0.15 0.5] Opened Control
    (Variables|Default|SetDotProduct 0.0)
    (bind _alpha (Timeline|Timeline Play)
      (:Update
        (Transformation|SetRelativeRotation (Variables|Default|GetDoorR) (Math|Rotator|MakeRotator 0.0 0.0 (Math|Float|Lerp 0.0 (Math|Float|SelectFloat 85.0 -85.0 (>= (Variables|Default|GetDotProduct) 0.0)) _alpha)) false false)
        (Transformation|SetRelativeRotation (Variables|Default|GetDoorL) (Math|Rotator|MakeRotator 0.0 0.0 (Math|Float|Lerp 0.0 (Math|Float|SelectFloat -85.0 85.0 (>= (Variables|Default|GetDotProduct) 0.0)) _alpha)) false false)
        (Audio|PlaySound2D "/Game/Sergio/Blueprints/UI/Sounds/SC_OpenJail.SC_OpenJail" 1.0 1.0 0.0 0 0)
        (Rendering|Components|Light|SetLightColor (Variables|Default|GetPointLight) (Variables|Default|GetLightColor_Open) true)
        (if (Math|Random|RandomBool)
          (Rendering|Components|Light|SetIntensity (Variables|Default|GetPointLight) (Math|Random|RandomFloatinRange 5e+01 1e+02))
          (else
            (Rendering|Components|Light|SetIntensity (Variables|Default|GetPointLight) (Math|Random|RandomFloatinRange 0.0 1e+02))
            (Utilities|FlowControl|Delay (Math|Random|RandomFloatinRange 0.0 0.3))))))
    (else
      (Variables|Default|SetDoorClosed? true))))

(event Custom|Auto%20Close
  ;[0.15 0.15 0.15 0.5] Irrelevant
)

(event Custom|DoorAutoClose
  ;[0.15 0.15 0.15 0.5] Irrelevant
)

(event EventBeginPlay
  (bind _asbp_third_person_character (Utilities|Casting|CastToBP_ThirdPersonCharacter (Game|GetPlayerCharacter 0)))
  (Variables|Default|SetPlayerRef _asbp_third_person_character)
  (Rendering|Components|Light|SetLightColor (Variables|Default|GetPointLight) (Variables|Default|GetLightColor) true)
  (if (Math|Random|RandomBool)
    (Rendering|Components|Light|SetIntensity (Variables|Default|GetPointLight) (Math|Random|RandomFloatinRange 5e+01 1e+02))
    (else
      (Rendering|Components|Light|SetIntensity (Variables|Default|GetPointLight) (Math|Random|RandomFloatinRange 0.0 1e+02) :!label _label)
      (Utilities|FlowControl|Delay (Math|Random|RandomFloatinRange 0.0 0.3))
      (goto _label))))

(event EventInteraction
  ;[0 0.02053 1 0.5] Door Animation
  (Audio|PlaySoundatLocation "/Game/Sergio/Blueprints/UI/Sounds/SC_MetalDoor.SC_MetalDoor" "0, 0, 0" "0, 0, 0" 1.0 1.0 0.0 0 0 0 0)
  (Timeline|Timeline_0 Stop))

(fn ConstructionScript)