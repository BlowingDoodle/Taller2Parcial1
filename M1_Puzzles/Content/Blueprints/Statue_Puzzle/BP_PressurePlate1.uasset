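; BP_PressurePlate1 is a statue puzzle pressure plate that activates while a BP_Statue overlaps its Box.
; Overlap begin and end toggle IsActive2 and swap the Cylinder material between active and pulse.
; Only begin overlap reports to BP_PPChecker actors, as plate ID 2, so deactivation is never sent.
; A separate CheckActivation event increments ActivePoints on a parent-actor BP_PPChecker and prints it.
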(event OnComponentBeginOverlap(Box)
  (params (OverlappedComponent :type Primitive%20Component%20Object%20Reference) (OtherActor :type Actor%20Object%20Reference) (OtherComp :type Primitive%20Component%20Object%20Reference) (OtherBodyIndex :type Integer) (bFromSweep :type Boolean) (SweepResult :type Hit%20Result%20Structure%20%28by%20ref%29))
  (Utilities|Casting|CastToBP_Statue OtherActor)
  (Variables|Default|SetIsActive2 true)
  (Rendering|Material|SetMaterial (Variables|Default|GetCylinder) 0 "/Game/StarterContent/Materials/M_Tech_Hex_Tile_Active.M_Tech_Hex_Tile_Active")
  (bind _outactors (Actor|GetAllActorsOfClass "/Game/Blueprints/Statue_Puzzle/BP_PPChecker.BP_PPChecker_C"))
  (Default|UpdatePressurePlateState _outactors 2 (Variables|Default|GetIsActive2)))

(event OnComponentEndOverlap(Box)
  (params (OverlappedComponent :type Primitive%20Component%20Object%20Reference) (OtherActor :type Actor%20Object%20Reference) (OtherComp :type Primitive%20Component%20Object%20Reference) (OtherBodyIndex :type Integer))
  (Utilities|Casting|CastToBP_Statue OtherActor)
  (Variables|Default|SetIsActive2 false)
  (Rendering|Material|SetMaterial (Variables|Default|GetCylinder) 0 "/Game/StarterContent/Materials/M_Tech_Hex_Tile_Pulse.M_Tech_Hex_Tile_Pulse"))

(event Custom|CheckActivation
  (bind _asbp_ppchecker (Utilities|Casting|CastToBP_PPChecker (Actor|GetParentActor)))
  (bind _output_get (Variables|/Game/Blueprints/Statue_Puzzle/BP_PPChecker.BP_PPChecker_C|SetActivePoints _asbp_ppchecker (+ (Variables|/Game/Blueprints/Statue_Puzzle/BP_PPChecker.BP_PPChecker_C|GetActivePoints _asbp_ppchecker) 1.0)))
  (Development|PrintString (Utilities|String|ToString(Float) _output_get)))

(event EventBeginPlay)

(event Collision|EventActorBeginOverlap
  (params (OtherActor :type Actor%20Object%20Reference)))

(event EventTick
  (params (DeltaSeconds :type Float%20%28single-precision%29)))

(fn ConstructionScript)